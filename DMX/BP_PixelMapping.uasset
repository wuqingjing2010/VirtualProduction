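; Pixel-mapping actor that drives DMX fixtures from what a SceneCapture2D sees.
; BeginPlay creates a render target at pixel-map size, and the capture and preview camera share one FOV setting.
; Each tick it steps through the fixture patches, pairing them with pixels in row order via persistent X/Y counters.
; Each pixel's color is converted to HSV, scaled to 0–255 and sent over DMX.
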(event `self.ReceiveBeginPlay`
  (bind _returnvalue (`KismetRenderingLibrary.CreateRenderTarget2D` (`self.PixelMap_Width`) (`self.PixelMap_Height`)))
  (set `SceneCaptureComponent2D.TextureTarget` _returnvalue (`self.SceneCaptureComponent2D`)))

(event `self.ReceiveTick`
  (params (DeltaSeconds :type "Float (single-precision)"))
  (`self.Set_PixelMap_Parameter`)
  (`self.Send_DMX_HSI` (`self.SceneCaptureComponent2D`) (`self.DMX_FixturePatchs`)))

(fn `Map_Fixture`
  (returns (X :type Integer) (Y :type Integer))
  (if (< (`self.Temp_X`) (`self.PixelMap_Width`))
    (set `self.Temp_X` (+ (`self.Temp_X`) 1))
    (return (- (`self.Temp_X`) 1) (- (`self.Temp_Y`) 1))
    (else
      (set `self.Temp_X` 1)
      (bind _output_get (set `self.Temp_Y` (+ (`self.Temp_Y`) 1)))
      (if (<= _output_get (`self.PixelMap_Height`))
        (return (- (`self.Temp_X`) 1) (- (`self.Temp_Y`) 1))))))

(fn `Send_DMX_HSI`
  (params (SceneCapture2D :type "SceneCaptureComponent2D Object Reference") (DMXFixturePatchs :type "Array of DMXEntityFixturePatchRef Structure"))
  (for _array_element DMXFixturePatchs
    (bind (_x _y) (`self.Map_Fixture`))
    (bind _returnvalue (`KismetRenderingLibrary.ReadRenderTargetRawPixel` (`SceneCaptureComponent2D.TextureTarget` SceneCapture2D) _x _y))
    (bind (_h _s _v) (`KismetMathLibrary.RGBToHSV` _returnvalue))
    (`DMXEntityFixturePatch.SendDMX` (`DMXEntityReferenceConversions.Conv_FixturePatchRefToObj` _array_element) (`|MakeMap` (struct :`Name` "Dimmer") (`KismetMathLibrary.FTrunc` (* 255 _v)) (struct :`Name` "HSB_Hue") (`KismetMathLibrary.FTrunc` (* _h 0.708333)) (struct :`Name` "HSB_Saturation") (`KismetMathLibrary.FTrunc` (* 255 _s)) :!type "DMXAttributeName Structure"))))

(fn `Set_PixelMap_Parameter`
  (bind _output_get (set `SceneCaptureComponent2D.FOVAngle` (`self.PixelMap_FOV`) (`self.SceneCaptureComponent2D`)))
  (`CameraComponent.SetFieldOfView` (`self.PixelMappingPreviewCam`) _output_get))

(fn `UserConstructionScript`
  (`self.Set_PixelMap_Parameter`))