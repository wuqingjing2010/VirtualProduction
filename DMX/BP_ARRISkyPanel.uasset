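; Blueprint for an ARRI SkyPanel light that sends its dimmer and color values over DMX through a fixture patch.
; The patch's active mode selects one of three supported layouts (temperature/tint, RGBW or hue/saturation), setting unused channels to -1 and printing an error for other modes.
; The mode check runs at construction and every Tick, where all nine values are then sent as one attribute map.
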(event `self.ReceiveBeginPlay`)

(event `self.ReceiveTick`
  (params (DeltaSeconds :type "Float (single-precision)"))
  (`self.Set_DMX_FixtureMode`)
  (`DMXEntityFixturePatch.SendDMX` (`DMXEntityReferenceConversions.Conv_FixturePatchRefToObj` (`self.DMX_FixturePatch`)) (`|MakeMap` (struct :`Name` "Dimmer") (`self.Dimmer`) (struct :`Name` "CTC") (`self.Temp`) (struct :`Name` "Tint") (`self.Tint`) (struct :`Name` "Red") (`self.Red`) (struct :`Name` "Green") (`self.Green`) (struct :`Name` "Blue") (`self.Blue`) (struct :`Name` "White") (`self.White`) (struct :`Name` "HSB_Hue") (`self.Hue`) (struct :`Name` "HSB_Saturation") (`self.Saturation`) :!type "DMXAttributeName Structure")))

(fn `Set_DMX_FixtureMode`
  (bind _activemode (`DMXEntityFixturePatch.ActiveMode` (`DMXEntityReferenceConversions.Conv_FixturePatchRefToObj` (`self.DMX_FixturePatch`))))
  (if (== _activemode 2)
    (set `self.DMX_FixtureMode` "NewEnumerator0")
    (set `self.Red` -1)
    (set `self.Green` -1)
    (set `self.Blue` -1)
    (set `self.White` -1)
    (set `self.Hue` -1)
    (set `self.Saturation` -1)
    (elif (== _activemode 6)
      (set `self.DMX_FixtureMode` "NewEnumerator1")
      (set `self.Temp` -1)
      (set `self.Tint` -1)
      (set `self.Hue` -1)
      (set `self.Saturation` -1)
      (elif (== _activemode 8)
        (set `self.DMX_FixtureMode` "NewEnumerator2")
        (set `self.Temp` -1)
        (set `self.Tint` -1)
        (set `self.Red` -1)
        (set `self.Green` -1)
        (set `self.Blue` -1)
        (set `self.White` -1)
        (else
          (`KismetSystemLibrary.PrintString` (`KismetStringLibrary.Concat_StrStr` "ERROR(" (`KismetSystemLibrary.GetDisplayName` self) "): Light Mode not supported!") true true (struct :`R` 1.0 :`G` 0.017204 :`A` 1.0)))))))

(fn `UserConstructionScript`
  (`self.Set_DMX_FixtureMode`))