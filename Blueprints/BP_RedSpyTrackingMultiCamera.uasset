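; Multi-camera tracking actor that drives a list of Cine Cameras from Live Link camera subjects.
; It refetches subject keys, including disabled ones, at construction and on Tick whenever their count differs from the camera count.
; Each Tick advances round-robin to one subject, enables it and copies only its frame transform to the camera at the same index.
; Optional debug printing shows one camera's transform and lens data, and invalid frames print an error.
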(event `self.ReceiveBeginPlay`)

(event `self.ReceiveTick`
  (params (DeltaSeconds :type "Float (single-precision)"))
  (bind _livelinksubjectkeys (`self.LiveLinkSubjectKeys`))
  (bind _printtime (`self.PrintTime`))
  (bind _returnvalue (`KismetArrayLibrary.Array_Length` _livelinksubjectkeys))
  (`self.getSubjectKeys`)
  (set `self.PrintTime` (* _returnvalue 0.0))
  (bind _output_get (set `self.CurrentCamera` (mod (+ (`self.CurrentCamera`) 1) _returnvalue)))
  (bind _output (`|GetArrayItem` _livelinksubjectkeys _output_get))
  (`LiveLinkBlueprintLibrary.SetLiveLinkSubjectEnabled` _output true)
  (bind _dataresult (`|EvaluateLiveLinkFrameWithSpecificRole` (`.SubjectName` (break `LiveLinkSubjectKey` _output)) "/Script/LiveLinkInterface.LiveLinkCameraRole")
    (:`then`
      (bind _output_2 (`|GetArrayItem` (`self.CineCameraLists`) _output_get))
      (`SceneComponent.K2_SetRelativeTransform` (`Actor.RootComponent` _output_2) (`.Transform` (break `LiveLinkCameraFrameData` (`.FrameData` (break `LiveLinkCameraBlueprintData` _dataresult)))) false false)
      ;[1 0.7683 0.5284] Print Debug Info
      (if (`self.PrintLiveLinkDebugInfo`)
        (if (== (`self.CurrentCamera`) (`self.CameraNumberToPrint`))
          (`KismetSystemLibrary.PrintString` (`KismetStringLibrary.Conv_VectorToString` (.scale (`.Transform` (break `LiveLinkCameraFrameData` (`.FrameData` (break `LiveLinkCameraBlueprintData` _dataresult)))))) true true (struct :`G` 0.66 :`B` 1.0 :`A` 1.0) _printtime)
          (`KismetSystemLibrary.PrintString` (`KismetStringLibrary.Conv_RotatorToString` (.rotation (`.Transform` (break `LiveLinkCameraFrameData` (`.FrameData` (break `LiveLinkCameraBlueprintData` _dataresult)))))) true true (struct :`G` 0.66 :`B` 1.0 :`A` 1.0) _printtime)
          (`KismetSystemLibrary.PrintString` (`KismetStringLibrary.Conv_VectorToString` (.location (`.Transform` (break `LiveLinkCameraFrameData` (`.FrameData` (break `LiveLinkCameraBlueprintData` _dataresult)))))) true true (struct :`G` 0.66 :`B` 1.0 :`A` 1.0) _printtime)
          (`KismetSystemLibrary.PrintString` (`KismetStringLibrary.Concat_StrStr` "Aspect Ratio: " (`KismetStringLibrary.Conv_DoubleToString` (`.AspectRatio` (break `LiveLinkCameraFrameData` (`.FrameData` (break `LiveLinkCameraBlueprintData` _dataresult))))) "Focal Length: " (`KismetStringLibrary.Conv_DoubleToString` (`.FocalLength` (break `LiveLinkCameraFrameData` (`.FrameData` (break `LiveLinkCameraBlueprintData` _dataresult))))) "Focus Distance: " (`KismetStringLibrary.Conv_DoubleToString` (`.FocusDistance` (break `LiveLinkCameraFrameData` (`.FrameData` (break `LiveLinkCameraBlueprintData` _dataresult)))))) true true (struct :`G` 0.66 :`B` 1.0 :`A` 1.0) _printtime)
          (`KismetSystemLibrary.PrintString` (`KismetStringLibrary.Concat_StrStr` "Camera: " (`KismetSystemLibrary.GetObjectName` _output_2)) true true (struct :`G` 0.66 :`B` 1.0 :`A` 1.0) _printtime))))
    (:`InvalidFrame`
      (`KismetSystemLibrary.PrintString` (`KismetStringLibrary.Concat_StrStr` "ERROR(" (`KismetSystemLibrary.GetDisplayName` self) "): Not Getting Live Link Data.") true true (struct :`R` 1.0 :`B` 0.066375 :`A` 1.0) (`self.PrintTime`)))))

(event `self.LiveLinkComponentController.OnLiveLinkUpdated`
  (params (DeltaTime :type "Float (single-precision)")))

(fn `getSubjectKeys`
  (if (!= (`KismetArrayLibrary.Array_Length` (`self.LiveLinkSubjectKeys`)) (`KismetArrayLibrary.Array_Length` (`self.CineCameraLists`)))
    (bind _returnvalue (`LiveLinkBlueprintLibrary.GetLiveLinkSubjects` true))
    (set `self.LiveLinkSubjectKeys` _returnvalue)))

(fn `UserConstructionScript`
  (`self.getSubjectKeys`))