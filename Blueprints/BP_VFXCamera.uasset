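; VFX cine camera Blueprint that matches real ARRI sensor formats and toggles a calibration grid.
; The construction script maps the selected camera model and format, covering LF and S35 variants, to a sensor width and height and applies them as the CineCamera filmback.
; Every Tick, ShowCalibGrid drives the calibrationDebug scalar in a Material Parameter Collection to show or hide the grid.
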(event `self.ReceiveBeginPlay`)

(event `self.ReceiveTick`
  (params (DeltaSeconds :type "Float (single-precision)"))
  (bind _materialparametercollection (`self.MaterialParameterCollection`))
  ;[1 1 1] Show or Hide Calibration Grid
  (if (`self.ShowCalibGrid`)
    (`KismetMaterialLibrary.SetScalarParameterValue` _materialparametercollection "calibrationDebug" 1.0)
    (else
      (`KismetMaterialLibrary.SetScalarParameterValue` _materialparametercollection "calibrationDebug"))))

(fn `UserConstructionScript`
  ;[1 1 1] Set Camera Sensor Size
  (switch `/Game/VirtualProduction/config/CameraModelsAndFormats` (`self.CameraModelsAndFormats`)
    (:`NewEnumerator0`
      (set `self.Censor_H` 25.540001)
      (set `self.Censor_W` 36.700001))
    (:`NewEnumerator2`
      (set `self.Censor_H` 15.31)
      (set `self.Censor_W` 36.700001))
    (:`NewEnumerator3`
      (set `self.Censor_H` 17.82)
      (set `self.Censor_W` 31.68))
    (:`NewEnumerator1`
      (set `self.Censor_H` 18.17)
      (set `self.Censor_W` 28.25))
    (:`NewEnumerator4`
      (set `self.Censor_H` 14.85)
      (set `self.Censor_W` 26.4))
    (:`NewEnumerator5`
      (set `self.Censor_H` 17.82)
      (set `self.Censor_W` 23.76))
    (:`NewEnumerator6`
      (set `self.Censor_H` 13.37)
      (set `self.Censor_W` 23.76)))
  (set `CineCameraComponent.Filmback` (make `CameraFilmbackSettings` (`self.Censor_W`) (`self.Censor_H`)) (`self.GetCineCameraComponent` self)))